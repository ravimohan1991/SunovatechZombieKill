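; Zombie spawner that keeps at most one live BP_ZombieCharacter of its own, spawning at its location when the player is nearby.
; Tick flags a respawn whenever the tracked zombie is invalid or dead.
; The flagged spawn waits until the player pawn is within VehicleDistanceLimit, then stores the new zombie and clears the flag.
; The construction script turns SpawnerText toward the player camera manager, without per-frame updates.
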(event EventTick
  (params (DeltaSeconds :type Float%20%28single-precision%29))
  (if (Utilities|IsValid (Variables|Default|GetCurrentZombie))
    (if (Class|SunovatechZombieKillZoCharacter|IsAlive (Variables|Default|GetCurrentZombie))
      _
      (else
        (Variables|Default|SetbShouldSpawnZombie true :!label _label)))
    (else
      (goto _label)))
  (if (Utilities|IsValid (Game|Player|GetPlayerPawn 0))
    (if (and (< (Math|Vector|VectorLength (- (Transformation|GetActorLocation (Game|Player|GetPlayerPawn 0)) (Transformation|GetActorLocation))) (Variables|Default|GetVehicleDistanceLimit)) (Variables|Default|GetbShouldSpawnZombie))
      (bind _returnvalue (Game|SpawnActorfromClass "/Game/AI/BP_ZombieCharacter.BP_ZombieCharacter_C" (Math|Conversions|ToTransform(Vector) (Transformation|GetActorLocation)) "Undefined" "MultiplyWithRoot" 0 0))
      (Variables|Default|SetbShouldSpawnZombie false)
      (Variables|Default|SetCurrentZombie _returnvalue))))

(fn ConstructionScript
  (bind _spawnertext (Variables|Default|GetSpawnerText))
  (Transformation|SetWorldRotation _spawnertext (Math|Rotator|FindLookatRotation (Transformation|GetWorldLocation _spawnertext) (Transformation|GetWorldLocation (Variables|/Script/Engine.PlayerCameraManager|GetTransformComponent (Variables|Default|GetPlayerCameraManager)))) false false))